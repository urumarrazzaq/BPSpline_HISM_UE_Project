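; BP_Label is a placeable label actor that pairs a static mesh with floating text.
; The construction script sets the text from LabelName, and two functions let callers change the text or swap the mesh.
; Every Tick it re-applies the text's relative offset and billboards it toward the player camera, using a look-at rotation computed from the actor's location.
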(event EventBeginPlay)

(event Collision|EventActorBeginOverlap
  (params (OtherActor :type Actor%20Object%20Reference)))

(event EventTick
  (params (DeltaSeconds :type Float%20%28single-precision%29))
  (Transformation|SetRelativeLocationAndRotation (Variables|Default|GetTextRender) (Variables|Default|GetTextRenderOffset) "0, 0, 0" false false)
  (Transformation|SetWorldRotation (Variables|Default|GetTextRender) (Math|Rotator|FindLookatRotation (Transformation|GetActorLocation) (Transformation|GetActorLocation (Game|GetPlayerCameraManager 0))) false false))

(fn ConstructionScript
  (Rendering|Components|TextRender|SetText (Variables|Default|GetTextRender) (Variables|Default|GetLabelName)))

(fn UpdateLabel
  (params (LabelName :type Text))
  (bind _output_get (Variables|Default|SetLabelName LabelName))
  (Rendering|Components|TextRender|SetText (Variables|Default|GetTextRender) _output_get))

(fn UpdateStaticMesh
  (params (NewMesh :type Static%20Mesh%20Object%20Reference))
  (Components|StaticMesh|SetStaticMesh (Variables|Default|GetStaticMesh) NewMesh))